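; Client-side soldier feedback component for a mutator, providing camera and audio effects for fatigue, dying, tinnitus and shell shock.
; Fatigue and dying events write saturation and vignette into the player camera manager's post-process settings, with IsDying stopping fatigue end from clearing the dying look.
; Dying end only clears that flag, while SoldierDead also resets post-processing and stops the deafen sound.
; Other events start or stop tinnitus audio and trigger the controller's shell shock.
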(event Custom|Soldier%20Dead
  (params (dead%20Soldier :type INS%20Soldier%20Object%20Reference%20%28by%20ref%29))
  ;[1 1 1] Dying And Tinnitus Module
  (Variables|Default|SetIsDying false)
  (bind _asinsplayer_camera_manager (Utilities|Casting|CastToINSPlayerCameraManager (Variables|/Script/Engine.PlayerController|GetPlayerCameraManager (Class|INSSoldier|GetPlayerController dead%20Soldier))))
  (Variables|/Script/Insurgency.INSPlayerCameraManager|SetPostProcessSettings _asinsplayer_camera_manager (Utilities|Struct|MakePostProcessSettings))
  (Class|INSSoldier|PlayCharacterSoundEvent dead%20Soldier "/Game/Audio/wwise/Sandstorm/Character/FX/Deafen/Stop_Deafen.Stop_Deafen" 0))

(event Custom|Stop%20Tinnitus%20To%20Client
  (params (Dying%20Soldier :type INS%20Soldier%20Object%20Reference%20%28by%20ref%29))
  ;[1 1 1] Tinnitus Module [On Client]
  (Class|INSSoldier|PlayCharacterSoundEvent Dying%20Soldier "/Game/Audio/wwise/Sandstorm/Character/FX/Deafen/Stop_Deafen.Stop_Deafen" 0))

(event Custom|Dying%20State%20Camera%20PostProcess%20Start
  (params (TargetController :type INS%20Player%20Controller%20Object%20Reference%20%28by%20ref%29))
  ;[1 1 1] Dying Module [On Client]
  (bind _asinsplayer_camera_manager (Utilities|Casting|CastToINSPlayerCameraManager (Variables|/Script/Engine.PlayerController|GetPlayerCameraManager TargetController)))
  (bind _structout (Utilities|Struct|SetmembersinPostProcessSettings (Variables|/Script/Insurgency.INSPlayerCameraManager|GetPostProcessSettings _asinsplayer_camera_manager) (Math|Vector4|MakeVector4 1.0 1.0 1.0 0.2) 1.0 0.5))
  (Variables|/Script/Insurgency.INSPlayerCameraManager|SetPostProcessSettings _asinsplayer_camera_manager _structout)
  (Variables|Default|SetIsDying true))

(event Custom|Dying%20State%20Camera%20PostProcess%20End
  (params (playerController :type INS%20Player%20Controller%20Object%20Reference%20%28by%20ref%29))
  ;[1 1 1] Dying Module [On Client]
  (Variables|Default|SetIsDying false))

(event Custom|Fatigue%20State%20Camera%20PostProcess%20Start
  (params (playerController :type INS%20Player%20Controller%20Object%20Reference%20%28by%20ref%29))
  ;[1 1 1] Fatigue Module [On Client]
  (bind _asinsplayer_camera_manager (Utilities|Casting|CastToINSPlayerCameraManager (Variables|/Script/Engine.PlayerController|GetPlayerCameraManager playerController)))
  (bind _structout (Utilities|Struct|SetmembersinPostProcessSettings (Variables|/Script/Insurgency.INSPlayerCameraManager|GetPostProcessSettings _asinsplayer_camera_manager) (Math|Vector4|MakeVector4 1.0 1.0 1.0 0.9) "(R=1.000000,G=0.500000,B=0.500000,A=0.500000)" 0.1))
  (Variables|/Script/Insurgency.INSPlayerCameraManager|SetPostProcessSettings _asinsplayer_camera_manager _structout))

(event Custom|Play%20Shell%20Shock%20To%20Client
  (params (soldier :type INS%20Soldier%20Object%20Reference%20%28by%20ref%29) (deafnessDuration :type Float%20%28single-precision%29))
  ;[1 1 1] Shell Shock Module
  (Class|INSPlayerController|PlayShellShock (Class|INSSoldier|GetPlayerController soldier) deafnessDuration))

(event Custom|Fatigue%20State%20Camera%20PostProcess%20End
  (params (playerController :type INS%20Player%20Controller%20Object%20Reference%20%28by%20ref%29))
  ;[1 1 1] Fatigue Module [On Client]
  (if (not (Variables|Default|GetIsDying))
    (bind _asinsplayer_camera_manager (Utilities|Casting|CastToINSPlayerCameraManager (Variables|/Script/Engine.PlayerController|GetPlayerCameraManager playerController)))
    (Variables|/Script/Insurgency.INSPlayerCameraManager|SetPostProcessSettings _asinsplayer_camera_manager (Utilities|Struct|MakePostProcessSettings))))

(event Custom|Play%20Tinnitus%20To%20Client
  (params (dyingSoldier :type INS%20Soldier%20Object%20Reference%20%28by%20ref%29))
  ;[1 1 1] Tinnitus Module [On Client]
  (Class|INSSoldier|PlayCharacterSoundEvent dyingSoldier "/Game/Audio/wwise/Sandstorm/Character/FX/Deafen/Play_Deafen.Play_Deafen" 0))

(event EventBeginPlay)

(event EventTick
  (params (DeltaSeconds :type Float%20%28single-precision%29)))