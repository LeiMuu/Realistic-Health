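; Movement ability control component for mutators that applies fatigue, healthy and dying penalties to a soldier's movement and weapon sway.
; Multicast events run the effects on clients: fatigue cancels sprint, drains stamina if sprinting and sets sway.
; Dying also cancels sprint, forces a crouch unless prone, empties stamina and sets sway.
; A flag tracks altered sway so the healthy event resets it only when needed.
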(event Custom|Multicast%20Dying%20State
  (params (soldier :type INS%20Soldier%20Object%20Reference%20%28by%20ref%29) (Sway%20Factor :type Float%20%28single-precision%29))
  ;[1 1 1] Dying Module [On Client]
  (Class|INSSoldier|CancelSprint soldier)
  (if (Class|INSSoldier|IsProne soldier)
    _
    (else
      (Character|Crouch soldier)))
  (Class|INSSoldier|SetStamina soldier 0.0)
  (Variables|/Script/Insurgency.INSSoldier|SetSwayFactor soldier Sway%20Factor)
  (Variables|Default|SetIsSwayIncrease true))

(event Custom|Multicast%20Healthy%20state
  (params (soldier :type INS%20Soldier%20Object%20Reference%20%28by%20ref%29))
  ;[1 1 1] Fatigue module [On Client]
  (if (Variables|Default|GetIsSwayIncrease)
    (Variables|/Script/Insurgency.INSSoldier|SetSwayFactor soldier 1.0)
    (Variables|Default|SetIsSwayIncrease false)))

(event Custom|Multicast%20Fatigue%20State
  (params (soldier :type INS%20Soldier%20Object%20Reference%20%28by%20ref%29) (drainStamina :type Float%20%28single-precision%29) (swayFactor :type Float%20%28single-precision%29))
  ;[1 1 1] Fatigue module [On Client]
  (if (Class|INSSoldier|IsSprinting soldier)
    (Class|INSSoldier|DrainStamina soldier drainStamina))
  (Class|INSSoldier|CancelSprint soldier)
  (Variables|/Script/Insurgency.INSSoldier|SetSwayFactor soldier swayFactor)
  (Variables|Default|SetIsSwayIncrease true))

(event EventBeginPlay)

(event EventTick
  (params (DeltaSeconds :type Float%20%28single-precision%29)))